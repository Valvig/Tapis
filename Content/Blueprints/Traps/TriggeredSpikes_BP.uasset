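; Spike trap that springs when the player enters its trigger and kills the player on contact with the spikes.
; After a configurable delay, a timeline moves the spike parent along relative Z with sweep.
; An optional alert-only flag makes both the triggering and the lethal contact work only while the game mode's Alert state is set.
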(event OnComponentBeginOverlap(SpikeParent)
  (params (OverlappedComponent :type Primitive%20Component%20Object%20Reference) (OtherActor :type Actor%20Object%20Reference) (OtherComp :type Primitive%20Component%20Object%20Reference) (OtherBodyIndex :type Integer) (bFromSweep :type Boolean) (SweepResult :type Hit%20Result%20Structure%20%28by%20ref%29))
  (bind _asplayer_character_tapis (Utilities|Casting|CastToPlayerCharacter_Tapis OtherActor))
  (if (Variables|Default|GetActiveOnAlertOnly?)
    (bind _asgame_mode_tapis (Utilities|Casting|CastToGameMode_Tapis (Game|GetGameMode)))
    (if (Variables|/Game/Blueprints/GameMode_Tapis.GameMode_Tapis_C|GetAlert _asgame_mode_tapis)
      (Default|Die _asplayer_character_tapis :!label _label))
    (else
      (goto _label))))

(event OnComponentBeginOverlap(Trigger)
  (params (OverlappedComponent :type Primitive%20Component%20Object%20Reference) (OtherActor :type Actor%20Object%20Reference) (OtherComp :type Primitive%20Component%20Object%20Reference) (OtherBodyIndex :type Integer) (bFromSweep :type Boolean) (SweepResult :type Hit%20Result%20Structure%20%28by%20ref%29))
  (Utilities|Casting|CastToPlayerCharacter_Tapis OtherActor)
  (if (Variables|Default|GetActiveOnAlertOnly?)
    (bind _asgame_mode_tapis (Utilities|Casting|CastToGameMode_Tapis (Game|GetGameMode)))
    (if (Variables|/Game/Blueprints/GameMode_Tapis.GameMode_Tapis_C|GetAlert _asgame_mode_tapis)
      (Utilities|FlowControl|Delay (Variables|Default|GetDelayTime) :!label _label)
      (CallFunction|Animate))
    (else
      (goto _label))))

(event Custom|Animate
  (bind _zvalue (Timeline|Animation PlayFromStart)
    (:Update
      (Transformation|SetRelativeLocation (Variables|Default|GetSpikeParent) (Math|Vector|MakeVector 0.0 0.0 _zvalue) true false))))

(fn ConstructionScript)