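; A saw-blade trap that spins while sweeping back and forth along a rail, killing the player on overlap and optionally destroying guards.
; A looping Move timeline lerps the blade between inset rail-bound ends, flipping direction on each finish, while Tick applies the spin.
; Optional flags hide the trap or blade and hold it dormant and harmless until Tick sees the game mode's Alert, then reveal and start it.
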(event OnComponentBeginOverlap(Blade)
  (params (OverlappedComponent :type Primitive%20Component%20Object%20Reference) (OtherActor :type Actor%20Object%20Reference) (OtherComp :type Primitive%20Component%20Object%20Reference) (OtherBodyIndex :type Integer) (bFromSweep :type Boolean) (SweepResult :type Hit%20Result%20Structure%20%28by%20ref%29))
  (bind _asplayer_character_tapis (Utilities|Casting|CastToPlayerCharacter_Tapis OtherActor)
    (:then
      (if (Variables|Default|GetActiveOnAlertOnly?)
        (bind _asgame_mode_tapis (Utilities|Casting|CastToGameMode_Tapis (Game|GetGameMode)))
        (if (Variables|/Game/Blueprints/GameMode_Tapis.GameMode_Tapis_C|GetAlert _asgame_mode_tapis)
          (Default|Die _asplayer_character_tapis :!label _label))
        (else
          (goto _label))))
    (:CastFailed
      (if (Variables|Default|GetCanKillGuards)
        (bind _asguard_parent_bp (Utilities|Casting|CastToGuardParent_BP OtherActor))
        (if (Variables|Default|GetActiveOnAlertOnly?)
          (bind _asgame_mode_tapis_2 (Utilities|Casting|CastToGameMode_Tapis (Game|GetGameMode)))
          (if (Variables|/Game/Blueprints/GameMode_Tapis.GameMode_Tapis_C|GetAlert _asgame_mode_tapis_2)
            (Actor|DestroyActor _asguard_parent_bp :!label _label_2))
          (else
            (goto _label_2)))))))

(event Custom|SpinBlade
  (bind _rightendofrail (Variables|Default|GetRightEndOfRail))
  (bind _blade (Variables|Default|GetBlade))
  (bind _leftendofrail (Variables|Default|GetLeftEndOfRail))
  (bind _relativelocation (Variables|/Script/Engine.SceneComponent|GetRelativeLocation _blade))
  (bind _value (Timeline|Move PlayFromStart)
    (:Update
      (if (Variables|Default|GetTurnAround)
        (Transformation|SetRelativeLocation (Variables|Default|GetBlade) (Math|Vector|MakeVector (.x (Math|Vector|Lerp(Vector) _leftendofrail _rightendofrail _value)) (.y _relativelocation) (.z (Math|Vector|Lerp(Vector) _leftendofrail _rightendofrail _value))) true false)
        (else
          (Transformation|SetRelativeLocation (Variables|Default|GetBlade) (Math|Vector|MakeVector (.x (Math|Vector|Lerp(Vector) _rightendofrail _leftendofrail _value)) (.y _relativelocation) (.z (Math|Vector|Lerp(Vector) _rightendofrail _leftendofrail _value))) true false))))
    (:Finished
      (if (Variables|Default|GetTurnAround)
        (Variables|Default|SetTurnAround false)
        (else
          (Variables|Default|SetTurnAround true)))
      (CallFunction|SpinBlade))))

(event EventBeginPlay
  (bind _rail (Variables|Default|GetRail))
  (bind _sawwidth (Variables|Default|GetSawWidth))
  (bind (_min _max) (Components|StaticMesh|GetLocalBounds _rail))
  (Variables|Default|SetLeftEndOfRail (+ _min (Math|Vector|MakeVector _sawwidth 0.0 0.0)))
  (Variables|Default|SetRightEndOfRail (- _max (Math|Vector|MakeVector _sawwidth 0.0 0.0)))
  (if (Variables|Default|GetVisibleOnAlertOnly?)
    (Rendering|SetVisibility (Variables|Default|GetDefaultSceneRoot) false true)
    (elif (Variables|Default|GetActiveOnAlertOnly?)
      (Rendering|SetVisibility (Variables|Default|GetBlade) false true)
      (else
        (Utilities|FlowControl|Delay (Variables|Default|GetFirstActivationDelay))
        (CallFunction|SpinBlade)))))

(event EventTick
  (params (DeltaSeconds :type Float%20%28single-precision%29))
  (if (Variables|Default|GetActiveOnAlertOnly?)
    (bind _asgame_mode_tapis (Utilities|Casting|CastToGameMode_Tapis (Game|GetGameMode)))
    (if (Variables|/Game/Blueprints/GameMode_Tapis.GameMode_Tapis_C|GetAlert _asgame_mode_tapis)
      (Variables|Default|SetActiveOnAlertOnly? false)
      (Rendering|SetVisibility (Variables|Default|GetDefaultSceneRoot) true true)
      (Utilities|FlowControl|Delay (Variables|Default|GetFirstActivationDelay))
      (CallFunction|SpinBlade))
    (else
      (Transformation|AddLocalRotation (Variables|Default|GetBlade) (Math|Rotator|MakeRotator (* DeltaSeconds (* 360 (Variables|Default|GetRevsPerSecond))) 0.0 0.0) false false))))

(fn ConstructionScript)