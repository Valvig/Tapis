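; Treadmill trap that carries the player, and optionally guards, along its forward vector and kills them on contact with its death box.
; Tick spins a cylinder and applies swept, delta-time-scaled offsets to actors overlapping the box.
; Flags can restrict movement and killing to the game mode's Alert state, hide the box until then, and let guards be moved or destroyed.
; The construction script counter-scales the arrow against actor scale.
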(event OnComponentBeginOverlap(DeathBox)
  (params (OverlappedComponent :type Primitive%20Component%20Object%20Reference) (OtherActor :type Actor%20Object%20Reference) (OtherComp :type Primitive%20Component%20Object%20Reference) (OtherBodyIndex :type Integer) (bFromSweep :type Boolean) (SweepResult :type Hit%20Result%20Structure%20%28by%20ref%29))
  (bind _asplayer_character_tapis (Utilities|Casting|CastToPlayerCharacter_Tapis OtherActor)
    (:then
      (if (Variables|Default|GetActiveOnAlertOnly?)
        (bind _asgame_mode_tapis (Utilities|Casting|CastToGameMode_Tapis (Game|GetGameMode)))
        (if (Variables|/Game/Blueprints/GameMode_Tapis.GameMode_Tapis_C|GetAlert _asgame_mode_tapis)
          (Default|Die _asplayer_character_tapis :!label _label))
        (else
          (goto _label))))
    (:CastFailed
      (if (Variables|Default|GetCanKillGuards)
        (bind _asguard_parent_bp (Utilities|Casting|CastToGuardParent_BP OtherActor))
        (if (Variables|Default|GetActiveOnAlertOnly?)
          (bind _asgame_mode_tapis_2 (Utilities|Casting|CastToGameMode_Tapis (Game|GetGameMode)))
          (if (Variables|/Game/Blueprints/GameMode_Tapis.GameMode_Tapis_C|GetAlert _asgame_mode_tapis_2)
            (Actor|DestroyActor _asguard_parent_bp :!label _label_2))
          (else
            (goto _label_2)))))))

(event EventBeginPlay
  (if (Variables|Default|GetVisibleOnAlertOnly?)
    (Rendering|SetVisibility (Variables|Default|GetBox) false true)))

(event EventTick
  (params (DeltaSeconds :type Float%20%28single-precision%29))
  (if (Variables|Default|GetActiveOnAlertOnly?)
    (bind _asgame_mode_tapis (Utilities|Casting|CastToGameMode_Tapis (Game|GetGameMode)))
    (if (Variables|/Game/Blueprints/GameMode_Tapis.GameMode_Tapis_C|GetAlert _asgame_mode_tapis)
      (if (Variables|Default|GetVisibleOnAlertOnly?)
        (Rendering|SetVisibility (Variables|Default|GetBox) true true))
      (Transformation|AddLocalRotation (Variables|Default|GetCylinder) "0.000000,1.000000, 0" false false :!label _label)
      (for _array_element (Collision|GetOverlappingActors (Variables|Default|GetBox) 0 :!class /Script/Engine.PrimitiveComponent)
        (bind _asplayer_character_tapis (Utilities|Casting|CastToPlayerCharacter_Tapis _array_element)
          (:then
            (Transformation|AddActorWorldOffset _asplayer_character_tapis (* (Math|Vector|GetForwardVector (Transformation|GetActorRotation)) (* DeltaSeconds (Variables|Default|GetMoveSpeed))) true :!label _label_2))
          (:CastFailed
            (if (Variables|Default|GetCanBeActivatedByGuards)
              (bind _asguard_parent_bp (Utilities|Casting|CastToGuardParent_BP _array_element))
              (goto _label_2))))))
    (else
      (goto _label))))

(fn ConstructionScript
  (Transformation|SetRelativeScale3D (Variables|Default|GetArrow) (/ "1.000000,1.000000,1.000000" (Transformation|GetActorScale3D))))