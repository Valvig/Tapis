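; Rolling stone trap that kills the player on overlap and can optionally destroy guards.
; A Move timeline sweeps the rock between the offset X ends of the Path bounds with curve-driven height, hides it, then repeats after a delay.
; Tick spins the rock, or for alert-only traps polls GameMode_Tapis for Alert to start rolling and reveal traps hidden until then.
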(event OnComponentBeginOverlap(Rock)
  (params (OverlappedComponent :type Primitive%20Component%20Object%20Reference) (OtherActor :type Actor%20Object%20Reference) (OtherComp :type Primitive%20Component%20Object%20Reference) (OtherBodyIndex :type Integer) (bFromSweep :type Boolean) (SweepResult :type Hit%20Result%20Structure%20%28by%20ref%29))
  (bind _asplayer_character_tapis (Utilities|Casting|CastToPlayerCharacter_Tapis OtherActor)
    (:then
      (if (Variables|Default|GetActiveOnAlertOnly?)
        (bind _asgame_mode_tapis (Utilities|Casting|CastToGameMode_Tapis (Game|GetGameMode)))
        (if (Variables|/Game/Blueprints/GameMode_Tapis.GameMode_Tapis_C|GetAlert _asgame_mode_tapis)
          (Default|Die _asplayer_character_tapis :!label _label))
        (else
          (goto _label))))
    (:CastFailed
      (if (Variables|Default|GetCanKillGuards)
        (bind _asguard_parent_bp (Utilities|Casting|CastToGuardParent_BP OtherActor))
        (if (Variables|Default|GetActiveOnAlertOnly?)
          (bind _asgame_mode_tapis_2 (Utilities|Casting|CastToGameMode_Tapis (Game|GetGameMode)))
          (if (Variables|/Game/Blueprints/GameMode_Tapis.GameMode_Tapis_C|GetAlert _asgame_mode_tapis_2)
            (Actor|DestroyActor _asguard_parent_bp :!label _label_2))
          (else
            (goto _label_2)))))))

(event Custom|RollStone
  (Rendering|SetVisibility (Variables|Default|GetRock) true true)
  (bind (_direction _value _zvalue) (Timeline|Move PlayFromStart)
    (:Update
      (Transformation|SetRelativeLocation (Variables|Default|GetRock) (Math|Vector|MakeVector (.x (Math|Vector|Lerp(Vector) (Variables|Default|GetLeftEndOfPath) (Variables|Default|GetRightEndOfPath) _value)) 0.0 (* _zvalue (Variables|Default|GetStartingHeight))) true false))
    (:Finished
      (Rendering|SetVisibility (Variables|Default|GetRock) false true)
      (Utilities|FlowControl|Delay (Variables|Default|GetDelayAppearingTime))
      (CallFunction|RollStone))))

(event EventBeginPlay
  (bind _path (Variables|Default|GetPath))
  (bind (_min _max) (Components|StaticMesh|GetLocalBounds _path))
  (bind (_x _y _z) (Math|Vector|BreakVector _max))
  (bind (_x_2 _y_2 _z_2) (Math|Vector|BreakVector _min))
  (Variables|Default|SetLeftEndOfPath (Math|Vector|MakeVector (- _x_2 (Variables|Default|GetLeftEndOffset)) _y_2 _z_2))
  (Variables|Default|SetRightEndOfPath (Math|Vector|MakeVector (+ _x (Variables|Default|GetRightEndOffset)) _y _z))
  (Variables|Default|SetStartingHeight (.z (Variables|/Script/Engine.SceneComponent|GetRelativeLocation (Variables|Default|GetRock))))
  (if (Variables|Default|GetVisibleOnAlertOnly?)
    (Rendering|SetVisibility (Variables|Default|GetDefaultSceneRoot) false true)
    (elif (not (Variables|Default|GetActiveOnAlertOnly?))
      (Utilities|FlowControl|Delay (Variables|Default|GetFirstActivationDelay))
      (CallFunction|RollStone))))

(event EventTick
  (params (DeltaSeconds :type Float%20%28single-precision%29))
  (if (Variables|Default|GetActiveOnAlertOnly?)
    (bind _asgame_mode_tapis (Utilities|Casting|CastToGameMode_Tapis (Game|GetGameMode)))
    (if (Variables|/Game/Blueprints/GameMode_Tapis.GameMode_Tapis_C|GetAlert _asgame_mode_tapis)
      (Variables|Default|SetActiveOnAlertOnly? false)
      (if (Variables|Default|GetVisibleOnAlertOnly?)
        (Rendering|SetVisibility (Variables|Default|GetDefaultSceneRoot) true true))
      (Utilities|FlowControl|Delay (Variables|Default|GetFirstActivationDelay))
      (CallFunction|RollStone))
    (else
      (Transformation|AddLocalRotation (Variables|Default|GetRock) (Math|Rotator|MakeRotator 0.0 0.0 (* DeltaSeconds (* 360 (Variables|Default|GetRevsPerSecond)))) false false))))

(fn ConstructionScript)