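; Spinning blade trap that kills the player on overlap and optionally destroys guards.
; Construction script spaces instanced blades radially, each with an overlap box attached.
; Timelines ramp rotation up and down and restore the initial rotation when switched off, while Tick sustains full spin and optional intervals toggle the trap.
; It can also stay dormant and hidden until the game mode raises an alert.
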(event Custom|HittedSomething
  (params (OverlappedComponent :type Primitive%20Component%20Object%20Reference) (OtherActor :type Actor%20Object%20Reference) (OtherComp :type Primitive%20Component%20Object%20Reference) (OtherBodyIndex :type Integer) (bFromSweep :type Boolean) (SweepResult :type Hit%20Result%20Structure%20%28by%20ref%29))
  (bind _asplayer_character_tapis (Utilities|Casting|CastToPlayerCharacter_Tapis OtherActor)
    (:then
      (Default|Die _asplayer_character_tapis))
    (:CastFailed
      (if (Variables|Default|GetCanKillGuards)
        (bind _asguard_parent_bp (Utilities|Casting|CastToGuardParent_BP OtherActor))
        (Actor|DestroyActor _asguard_parent_bp)))))

(event Custom|TurnOn
  (bind _blades (Variables|Default|GetBlades))
  (Collision|SetCollisionEnabled (Variables|Default|GetPole) "NoCollision")
  (Collision|SetCollisionEnabled (Variables|Default|GetBlades) "NoCollision")
  (Variables|Default|SetIsOn true)
  (for _array_element (Variables|Default|GetCollisionBoxes)
    (Collision|SetCollisionEnabled _array_element "QueryOnly"))
  (bind (_direction _playingrate) (Timeline|TurningOn PlayFromStart)
    (:Update
      (Transformation|AddRelativeRotation (Variables|Default|GetBlades) (Math|Rotator|MakeRotator 0.0 0.0 (* _playingrate (* (Utilities|Time|GetWorldDeltaSeconds) (* (Variables|Default|GetRotationMultiplier) (Variables|Default|GetRevsPerSeconds))))) false false))
    (:Finished
      (if (Variables|Default|GetIsOn)
        _
        (else
          (bind _value (Timeline|ReturnToNormal PlayFromStart)
            (:Update
              (Transformation|SetRelativeRotation (Variables|Default|GetBlades) (Math|Rotator|Lerp(Rotator) (Variables|/Script/Engine.SceneComponent|GetRelativeRotation (Variables|Default|GetBlades)) (Variables|Default|GetInitialRotation) _value) true false)))))
      (if (Utilities|Enum|Equal(Enum) _direction "Forward")
        (Variables|Default|SetIsSpinning true)
        (Collision|SetCollisionEnabled _blades "NoCollision")
        (if (Variables|Default|GetUseIntervals)
          (Utilities|FlowControl|Delay (Variables|Default|GetStateTimeInterval))
          (CallFunction|TurnOff))
        (else
          (Variables|Default|SetIsSpinning false)
          (Collision|SetCollisionEnabled _blades "QueryAndPhysics")
          (for _array_element_2 (Variables|Default|GetCollisionBoxes)
            (Collision|SetCollisionEnabled _array_element_2 "NoCollision"))
          (if (Variables|Default|GetUseIntervals)
            (Utilities|FlowControl|Delay (Variables|Default|GetStateTimeInterval))
            (CallFunction|Turnon)))))))

(event Custom|TurnOff
  (bind _blades (Variables|Default|GetBlades))
  (Collision|SetCollisionEnabled (Variables|Default|GetPole) "NoCollision")
  (Collision|SetCollisionEnabled (Variables|Default|GetBlades) "NoCollision")
  (Variables|Default|SetIsOn false)
  (bind (_direction _playingrate) (Timeline|TurningOn ReverseFromEnd)
    (:Update
      (Transformation|AddRelativeRotation (Variables|Default|GetBlades) (Math|Rotator|MakeRotator 0.0 0.0 (* _playingrate (* (Utilities|Time|GetWorldDeltaSeconds) (* (Variables|Default|GetRotationMultiplier) (Variables|Default|GetRevsPerSeconds))))) false false))
    (:Finished
      (if (Variables|Default|GetIsOn)
        _
        (else
          (bind _value (Timeline|ReturnToNormal PlayFromStart)
            (:Update
              (Transformation|SetRelativeRotation (Variables|Default|GetBlades) (Math|Rotator|Lerp(Rotator) (Variables|/Script/Engine.SceneComponent|GetRelativeRotation (Variables|Default|GetBlades)) (Variables|Default|GetInitialRotation) _value) true false)))))
      (if (Utilities|Enum|Equal(Enum) _direction "Forward")
        (Variables|Default|SetIsSpinning true)
        (Collision|SetCollisionEnabled _blades "NoCollision")
        (if (Variables|Default|GetUseIntervals)
          (Utilities|FlowControl|Delay (Variables|Default|GetStateTimeInterval))
          (CallFunction|TurnOff))
        (else
          (Variables|Default|SetIsSpinning false)
          (Collision|SetCollisionEnabled _blades "QueryAndPhysics")
          (for _array_element (Variables|Default|GetCollisionBoxes)
            (Collision|SetCollisionEnabled _array_element "NoCollision"))
          (if (Variables|Default|GetUseIntervals)
            (Utilities|FlowControl|Delay (Variables|Default|GetStateTimeInterval))
            (CallFunction|Turnon)))))))

(event EventBeginPlay
  (if (Variables|Default|GetRotateClockwise)
    (Variables|Default|SetRotationMultiplier 360)
    (else
      (Variables|Default|SetRotationMultiplier -360)))
  (for _array_element (Variables|Default|GetCollisionBoxes)
    (Collision|BindEventtoOnComponentBeginOverlap _array_element (delegate Custom|HittedSomething)))
  (Variables|Default|SetInitialRotation (Variables|/Script/Engine.SceneComponent|GetRelativeRotation (Variables|Default|GetBlades)))
  (if (Variables|Default|GetActiveOnAlertOnly?)
    (if (Variables|Default|GetVisibleOnAlertOnly?)
      (Rendering|SetVisibility (Variables|Default|GetDefaultSceneRoot) false true)
      (else
        (Rendering|SetVisibility (Variables|Default|GetBlades) false false)))
    (Collision|SetCollisionEnabled (Variables|Default|GetPole) "NoCollision")
    (Collision|SetCollisionEnabled (Variables|Default|GetBlades) "NoCollision")
    (elif (not (Variables|Default|GetVisibleOnAlertOnly?))
      (if (Variables|Default|GetIsOn)
        (CallFunction|Turnon)))))

(event EventTick
  (params (DeltaSeconds :type Float%20%28single-precision%29))
  (if (Variables|Default|GetActiveOnAlertOnly?)
    (bind _asgame_mode_tapis (Utilities|Casting|CastToGameMode_Tapis (Game|GetGameMode)))
    (if (Variables|/Game/Blueprints/GameMode_Tapis.GameMode_Tapis_C|GetAlert _asgame_mode_tapis)
      (Variables|Default|SetActiveOnAlertOnly? false)
      (Rendering|SetVisibility (Variables|Default|GetDefaultSceneRoot) true true)
      (if (Variables|Default|GetIsOn)
        (CallFunction|Turnon)))
    (elif (and (Variables|Default|GetIsOn) (Variables|Default|GetIsSpinning))
      (Transformation|AddRelativeRotation (Variables|Default|GetBlades) (Math|Rotator|MakeRotator 0.0 0.0 (* DeltaSeconds (* (Variables|Default|GetRotationMultiplier) (Variables|Default|GetRevsPerSeconds)))) false false))))

(fn ConstructionScript
  (bind _blades (Variables|Default|GetBlades))
  (bind _r (Variables|Default|GetR))
  (bind _numberofblades (Variables|Default|GetNumberOfBlades))
  (bind _blades_2 (Variables|Default|GetBlades))
  (bind _returnvalue (Transformation|GetRelativeTransform _blades_2))
  (bind (_min _max) (Components|StaticMesh|GetLocalBounds _blades))
  (bind (_location _rotation _scale) (Math|Transform|BreakTransform _returnvalue))
  (for _index (range 0 (- _numberofblades 1))
    (Variables|Default|SetAngle (+ (* _index (/ 3.6e+02 (Math|Conversions|ToFloat(Integer) _numberofblades))) 9e+01))
    (Components|InstancedStaticMesh|AddInstance (Variables|Default|GetBlades) (Math|Transform|MakeTransform (Math|Vector|MakeVector (.x _location) (.y _location) (- (.z _location) 105.0)) (Math|Rotator|CombineRotators _rotation (Math|Rotator|MakeRotator 0.0 0.0 (* _index (/ 3.6e+02 (Math|Conversions|ToFloat(Integer) _numberofblades))))) _scale))
    (bind _returnvalue_2 (AddComponent|AddBoxComponent false (Math|Transform|MakeTransform (Math|Vector|MakeVector (.x _location) (.y _location) (- (.z _location) 105.0)) (Math|Rotator|CombineRotators _rotation (Math|Rotator|MakeRotator 0.0 0.0 (* _index (/ 3.6e+02 (Math|Conversions|ToFloat(Integer) _numberofblades))))) _scale)))
    (Collision|SetCollisionEnabled _returnvalue_2 "NoCollision")
    (Utilities|Array|Add (Variables|Default|GetCollisionBoxes) _returnvalue_2)
    (Transformation|AttachComponentToComponent _returnvalue_2 (Variables|Default|GetBlades) "None" "KeepRelative" "KeepRelative" "KeepRelative" true)
    (Components|Box|SetBoxExtent _returnvalue_2 (+ (/ (+ (* _min -1) _max) 2.0) (Variables|Default|GetModifyBoxExtentBy)) true)
    (Transformation|SetRelativeLocation _returnvalue_2 (Math|Vector|MakeVector (* _r (Math|Trig|Sin(Degrees) (Variables|Default|GetAngle))) (* (* (Math|Trig|Cos(Degrees) (Variables|Default|GetAngle)) _r) -1.0) -5.0) false false)))