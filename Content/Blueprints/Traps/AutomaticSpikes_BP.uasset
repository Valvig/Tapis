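; AutomaticSpikes_BP is a trap whose spikes move on their own in a repeating cycle and kill the player on contact.
; From BeginPlay, a timeline drives SpikeParent's relative Z with sweep, then waits DelayTime and replays itself in an endless loop.
; Any overlap with SpikeParent casts the other actor to PlayerCharacter_Tapis and calls Die on it.
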(event OnComponentBeginOverlap(SpikeParent)
  (params (OverlappedComponent :type Primitive%20Component%20Object%20Reference) (OtherActor :type Actor%20Object%20Reference) (OtherComp :type Primitive%20Component%20Object%20Reference) (OtherBodyIndex :type Integer) (bFromSweep :type Boolean) (SweepResult :type Hit%20Result%20Structure%20%28by%20ref%29))
  (bind _asplayer_character_tapis (Utilities|Casting|CastToPlayerCharacter_Tapis OtherActor))
  (Default|Die _asplayer_character_tapis))

(event Custom|Animate
  (bind _zvalue (Timeline|Animation PlayFromStart)
    (:Update
      (Transformation|SetRelativeLocation (Variables|Default|GetSpikeParent) (Math|Vector|MakeVector 0.0 0.0 _zvalue) true false))
    (:Finished
      (Utilities|FlowControl|Delay (Variables|Default|GetDelayTime))
      (CallFunction|Animate))))

(event EventBeginPlay
  (CallFunction|Animate))

(fn ConstructionScript)