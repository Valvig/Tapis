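; RedLight is a rotating alarm light prop that switches on while the game mode's Alert flag is set.
; Each tick it checks GameMode_Tapis and, during an alert, shows both spotlights.
; A Rotate timeline spins the root yaw a full turn from its starting rotation, with a Restart flag replaying it each time it finishes.
; Nothing here hides the lights again when the alert ends.
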(event EventTick
  (params (DeltaSeconds :type Float%20%28single-precision%29))
  (bind _asgame_mode_tapis (Utilities|Casting|CastToGameMode_Tapis (Game|GetGameMode)))
  (if (Variables|/Game/Blueprints/GameMode_Tapis.GameMode_Tapis_C|GetAlert _asgame_mode_tapis)
    (Rendering|SetVisibility (Variables|Default|GetSpotLight1) true false)
    (Rendering|SetVisibility (Variables|Default|GetSpotLight) true false)
    (if (Variables|Default|GetRestart)
      (bind _angle (Timeline|Rotate PlayFromStart)
        (:Update
          (Variables|Default|SetRestart false)
          (Transformation|SetRelativeRotation (Variables|Default|GetDefaultSceneRoot) (Math|Rotator|MakeRotator 0.0 0.0 (+ (* _angle 3.6e+02) (Variables|Default|GetStartRotation))) false false))
        (:Finished
          (Variables|Default|SetRestart true))))))

(event EventBeginPlay
  (Variables|Default|SetStartRotation (.yaw (Transformation|GetWorldRotation (Variables|Default|GetDefaultSceneRoot)))))

(fn ConstructionScript)