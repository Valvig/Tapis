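; WinBox is an interactible that acts as the level's win trigger.
; On BeginPlay it copies its NextLevel value into GameMode_Tapis.
; When PlayerCharacter_Tapis overlaps it while the game mode's Alert flag is true, it sets Win on TapisGameInstance and opens GameOver_map.
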(event EventBeginPlay
  (bind _asgame_mode_tapis (Utilities|Casting|CastToGameMode_Tapis (Game|GetGameMode)))
  (Variables|/Game/Blueprints/GameMode_Tapis.GameMode_Tapis_C|SetNextLevel _asgame_mode_tapis (Variables|Default|GetNextLevel)))

(event Collision|EventActorBeginOverlap
  (params (OtherActor :type Actor%20Object%20Reference))
  (Utilities|Casting|CastToPlayerCharacter_Tapis OtherActor)
  (bind _asgame_mode_tapis (Utilities|Casting|CastToGameMode_Tapis (Game|GetGameMode)))
  (if (Variables|/Game/Blueprints/GameMode_Tapis.GameMode_Tapis_C|GetAlert _asgame_mode_tapis)
    ;[0 0.4735 0.3478] Win
    (bind _astapis_game_instance (Utilities|Casting|CastToTapisGameInstance (Game|GetGameInstance)))
    (Variables|/Game/Blueprints/GameInstance/TapisGameInstance.TapisGameInstance_C|SetWin _astapis_game_instance true)
    (Game|OpenLevel(byName) "GameOver_map")))

(fn ConstructionScript)