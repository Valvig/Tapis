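; Blueprint for a stoppable moving door that toggles between its start position and an end point when the Tapis player character enters its touch trigger.
; BeginPlay caches both positions, and each overlap alternately plays or reverses a timeline from its current progress.
; The timeline lerps the door's world location between them with sweep enabled, so blocking collision can stop the movement.
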(event OnComponentBeginOverlap(playerTouch)
  (params (OverlappedComponent :type Primitive%20Component%20Object%20Reference) (OtherActor :type Actor%20Object%20Reference) (OtherComp :type Primitive%20Component%20Object%20Reference) (OtherBodyIndex :type Integer) (bFromSweep :type Boolean) (SweepResult :type Hit%20Result%20Structure%20%28by%20ref%29))
  (Utilities|Casting|CastToPlayerCharacter_Tapis OtherActor)
  (if (Variables|Default|GetHasAlreadyMoved)
    (Variables|Default|SetHasAlreadyMoved false)
    (bind _newtrack_0 (Timeline|Timeline_0 Reverse)
      (:Update
        (Transformation|SetWorldLocation (Variables|Default|Getdoor) (Math|Vector|Lerp(Vector) (Variables|Default|GetstartLocation) (Variables|Default|GetendLocation) _newtrack_0) true false)))
    (else
      (Variables|Default|SetHasAlreadyMoved true)
      (Timeline|Timeline_0 Play))))

(event EventBeginPlay
  (Variables|Default|SetstartLocation (Transformation|GetWorldLocation (Variables|Default|Getdoor)))
  (Variables|Default|SetendLocation (Transformation|GetWorldLocation (Variables|Default|GetendPoint))))

(fn ConstructionScript)