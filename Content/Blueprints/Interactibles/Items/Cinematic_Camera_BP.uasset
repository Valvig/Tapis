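; Cinematic camera trigger that blends the player's view to this actor's camera and shows a text panel when PlayerCharacter_Tapis overlaps its box.
; It flags the player as in a cinematic, disables input and movement, then waits out the cubic blend before creating Cinematic_PanelForText with this instance's text index.
; After a short delay it clears the flag and re-enables input, but does not restore movement mode or view target itself.
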(event OnComponentBeginOverlap(Box)
  (params (OverlappedComponent :type Primitive%20Component%20Object%20Reference) (OtherActor :type Actor%20Object%20Reference) (OtherComp :type Primitive%20Component%20Object%20Reference) (OtherBodyIndex :type Integer) (bFromSweep :type Boolean) (SweepResult :type Hit%20Result%20Structure%20%28by%20ref%29))
  (bind _asplayer_character_tapis (Utilities|Casting|CastToPlayerCharacter_Tapis OtherActor))
  (Variables|/Game/Blueprints/Player/PlayerCharacter_Tapis.PlayerCharacter_Tapis_C|SetIsinCinematic _asplayer_character_tapis true)
  (Input|DisableInput (Game|GetPlayerCharacter 0) (Game|GetPlayerController 0))
  (Game|Player|SetViewTargetwithBlend (Game|GetPlayerController 0) (Components|GetOwner (Variables|Default|GetCamera)) 2.0 "VTBlend_Cubic" 1.0 true)
  (Pawn|Components|CharacterMovement|SetMovementMode (Variables|/Script/Engine.Character|GetCharacterMovement (Game|GetPlayerCharacter 0)) "MOVE_None" 0)
  (Utilities|FlowControl|Delay 2.0)
  (bind _returnvalue (UserInterface|CreateWidget "/Game/Blueprints/Player/HUDWidgets/Cinematic_PanelForText.Cinematic_PanelForText_C" (Game|GetPlayerController 0)))
  (Variables|/Game/Blueprints/Player/HUDWidgets/Cinematic_PanelForText.Cinematic_PanelForText_C|SetIndex _returnvalue (Variables|Default|GetWhichTextBlockShouldIRead))
  (bind _asplayer_character_tapis_2 (Utilities|Casting|CastToPlayerCharacter_Tapis OtherActor))
  (bind _output_get (Variables|/Game/Blueprints/Player/PlayerCharacter_Tapis.PlayerCharacter_Tapis_C|SetHUD%20Cinematic%20Ref _asplayer_character_tapis_2 _returnvalue))
  (UserInterface|Viewport|AddtoViewport _output_get 0)
  (Utilities|FlowControl|Delay 1.0)
  (bind _asplayer_character_tapis_3 (Utilities|Casting|CastToPlayerCharacter_Tapis OtherActor))
  (Variables|/Game/Blueprints/Player/PlayerCharacter_Tapis.PlayerCharacter_Tapis_C|SetIsinCinematic _asplayer_character_tapis_3 false)
  (Input|EnableInput (Game|GetPlayerCharacter 0) (Game|GetPlayerController 0)))

(fn ConstructionScript)