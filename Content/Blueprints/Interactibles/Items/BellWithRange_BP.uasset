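; BellWithRange_BP is an interactible bell that alerts guards within hearing range when rung.
; ItemAction plays the sound, calls ReactToSound on every GuardParent_BP overlapping the VisibleRangeOfSound sphere, then runs a swing timeline.
; The timeline swings the bell and DingDing in opposite directions, holds the rope's world rotation at zero, and blocks reuse until finished.
; The construction script sizes the sphere from RangeOfSound.
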(event EventItemAction
  (if (Variables|Default|GetCanUseAgain)
    (Audio|PlaySoundatLocation "/Game/Sounds/BELL.BELL" (Transformation|GetWorldLocation (Variables|Default|GetBell)) "0, 0, 0" 0.5 1.0 0.0 0 0 0)
    (Variables|Default|SetCanUseAgain false)
    (for _array_element (Collision|GetOverlappingActors (Variables|Default|GetVisibleRangeOfSound) "/Game/Blueprints/Guards/GuardParent_BP.GuardParent_BP_C" :!class /Script/Engine.PrimitiveComponent)
      (bind _asguard_parent_bp (Utilities|Casting|CastToGuardParent_BP _array_element))
      (Default|ReacttoSound _asguard_parent_bp self))
    (bind _valuebell (Timeline|AnimateBell PlayFromStart)
      (:Update
        (Transformation|SetRelativeRotation (Variables|Default|GetBell) (Math|Rotator|Lerp(Rotator) "0, 0,25.000000" "0, 0,-25.000000" _valuebell) false false)
        (Transformation|SetRelativeRotation (Variables|Default|GetDingDing) (Math|Rotator|Lerp(Rotator) "0, 0,-20.000000" "0, 0,20.000000" _valuebell) false false)
        (Transformation|SetWorldRotation (Variables|Default|GetRope) "0, 0, 0" false false))
      (:Finished
        (Variables|Default|SetCanUseAgain true)))))

(fn ConstructionScript
  (|CallParentFunction)
  (Components|Sphere|SetSphereRadius (Variables|Default|GetVisibleRangeOfSound) (Variables|Default|GetRangeOfSound) true))