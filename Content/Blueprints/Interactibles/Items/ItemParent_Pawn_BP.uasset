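; Base pawn Blueprint for interactible items that the player character can use when standing nearby.
; An angled widget component is initialized with its owning item and the item state.
; Box overlap toggles the state and the player's interact flag, registering the item as closest on entry.
; ItemAction is a placeholder that only prints a no-function message, apparently intended for child Blueprints to override.
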(event OnComponentBeginOverlap(Box)
  (params (OverlappedComponent :type Primitive%20Component%20Object%20Reference) (OtherActor :type Actor%20Object%20Reference) (OtherComp :type Primitive%20Component%20Object%20Reference) (OtherBodyIndex :type Integer) (bFromSweep :type Boolean) (SweepResult :type Hit%20Result%20Structure%20%28by%20ref%29))
  ;[0.6087 0.2126 0] CanInteract
  (Utilities|Casting|CastToPlayerCharacter_Tapis OtherActor)
  (Variables|Default|SetItemState "NewEnumerator1")
  (bind _asplayer_character_tapis (Utilities|Casting|CastToPlayerCharacter_Tapis (Game|GetPlayerCharacter 0)))
  (Variables|/Game/Blueprints/Player/PlayerCharacter_Tapis.PlayerCharacter_Tapis_C|SetClosestItem _asplayer_character_tapis self)
  (Variables|/Game/Blueprints/Player/PlayerCharacter_Tapis.PlayerCharacter_Tapis_C|SetCanInteract _asplayer_character_tapis true))

(event OnComponentEndOverlap(Box)
  (params (OverlappedComponent :type Primitive%20Component%20Object%20Reference) (OtherActor :type Actor%20Object%20Reference) (OtherComp :type Primitive%20Component%20Object%20Reference) (OtherBodyIndex :type Integer))
  ;[0.6087 0.2126 0] CanInteract
  (Utilities|Casting|CastToPlayerCharacter_Tapis OtherActor)
  (Variables|Default|SetItemState "NewEnumerator0")
  (bind _asplayer_character_tapis (Utilities|Casting|CastToPlayerCharacter_Tapis (Game|GetPlayerCharacter 0)))
  (Variables|/Game/Blueprints/Player/PlayerCharacter_Tapis.PlayerCharacter_Tapis_C|SetCanInteract _asplayer_character_tapis false))

(event Custom|ItemAction
  (Development|PrintString "Cet objet n'a pas de fonction associée."))

(event EventBeginPlay
  ;[0.04831 0.773 0] WidgetSetup
  (bind _asitem_state_widget (Utilities|Casting|CastToItemStateWidget (UserInterface|GetUserWidgetObject (Variables|Default|GetItemWidget))))
  (Variables|/Game/Blueprints/Interactibles/Widget/ItemStateWidget.ItemStateWidget_C|SetOwner _asitem_state_widget self)
  (Variables|/Game/Blueprints/Interactibles/Widget/ItemStateWidget.ItemStateWidget_C|SetItemState _asitem_state_widget (Variables|Default|GetItemState))
  (Transformation|SetWorldRotation (Variables|Default|GetItemWidget) (Math|Rotator|MakeRotator 0.0 45.0 1.8e+02) false false))

(fn ConstructionScript)