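; Treasure pickup item: a bobbing RavenStone that, when taken, raises the game mode's Alert flag.
; A self-restarting timeline animates the stone's height until it is taken.
; ItemAction either collects it immediately or, with Cutscene set, blends to a camera and shows an indexed cinematic text panel.
; After the cutscene, Tick waits for PromptQuitted, then destroys the stone and item widget and disables itself.
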(event Custom|Animate
  (bind _value (Timeline|Float PlayFromStart)
    (:Update
      (if (not (Variables|Default|GetTaken))
        (Transformation|SetRelativeLocation (Variables|Default|GetRavenStone) (Math|Vector|MakeVector 0.0 0.0 (Math|Float|Lerp 28.0 31.0 _value)) true false)))
    (:Finished
      (if (not (Variables|Default|GetTaken))
        (CallFunction|Animate)))))

(event EventBeginPlay
  (|CallParentFunction)
  (CallFunction|Animate))

(event EventTick
  (params (DeltaSeconds :type Float%20%28single-precision%29))
  (|CallParentFunction DeltaSeconds)
  (if (not (Variables|Default|GetCutscene))
    (if (Variables|Default|GetPromptQuitted)
      (Components|DestroyComponent (Variables|Default|GetRavenStone))
      (Variables|Default|SetTaken true)
      (bind _asgame_mode_tapis (Utilities|Casting|CastToGameMode_Tapis (Game|GetGameMode)))
      (Variables|/Game/Blueprints/GameMode_Tapis.GameMode_Tapis_C|SetAlert _asgame_mode_tapis true)
      (bind _asplayer_character_tapis (Utilities|Casting|CastToPlayerCharacter_Tapis (Game|GetPlayerCharacter 0)))
      (Variables|/Game/Blueprints/Player/PlayerCharacter_Tapis.PlayerCharacter_Tapis_C|SetPromptQuitted _asplayer_character_tapis false)
      (Actor|Tick|SetActorTickEnabled false)
      (Components|DestroyComponent (Variables|Default|GetItemWidget)))))

(event EventItemAction
  (bind _returnvalue (Game|GetPlayerCharacter 0))
  (Pawn|Components|CharacterMovement|SetMovementMode (Variables|/Script/Engine.Character|GetCharacterMovement (Game|GetPlayerCharacter 0)) "MOVE_None" 0)
  (EventDispatchers|UnbindallEventsfromOnComponentEndOverlap (Variables|Default|GetBox))
  (bind _asplayer_character_tapis (Utilities|Casting|CastToPlayerCharacter_Tapis (Game|GetPlayerCharacter 0)))
  (Variables|/Game/Blueprints/Player/PlayerCharacter_Tapis.PlayerCharacter_Tapis_C|SetCanInteract _asplayer_character_tapis false)
  (Variables|Default|SetItemState "NewEnumerator2")
  (if (Variables|Default|GetCutscene)
    (bind _asplayer_character_tapis_2 (Utilities|Casting|CastToPlayerCharacter_Tapis _returnvalue))
    (Variables|/Game/Blueprints/Player/PlayerCharacter_Tapis.PlayerCharacter_Tapis_C|SetIsinCinematic _asplayer_character_tapis_2 true)
    (Input|DisableInput (Game|GetPlayerCharacter 0) (Game|GetPlayerController 0))
    (Game|Player|SetViewTargetwithBlend (Game|GetPlayerController 0) (Components|GetOwner (Variables|Default|GetCamera)) 2.0 "VTBlend_Cubic" 1.0 true)
    (Pawn|Components|CharacterMovement|SetMovementMode (Variables|/Script/Engine.Character|GetCharacterMovement (Game|GetPlayerCharacter 0)) "MOVE_None" 0)
    (Utilities|FlowControl|Delay 2.0)
    (bind _returnvalue_2 (UserInterface|CreateWidget "/Game/Blueprints/Player/HUDWidgets/Cinematic_PanelForText.Cinematic_PanelForText_C" (Game|GetPlayerController 0)))
    (Variables|/Game/Blueprints/Player/HUDWidgets/Cinematic_PanelForText.Cinematic_PanelForText_C|SetIndex _returnvalue_2 (Variables|Default|GetWhichTextBlockShouldIRead))
    (bind _asplayer_character_tapis_3 (Utilities|Casting|CastToPlayerCharacter_Tapis _returnvalue))
    (bind _output_get (Variables|/Game/Blueprints/Player/PlayerCharacter_Tapis.PlayerCharacter_Tapis_C|SetHUD%20Cinematic%20Ref _asplayer_character_tapis_3 _returnvalue_2))
    (UserInterface|Viewport|AddtoViewport _output_get 0)
    (Utilities|FlowControl|Delay 1.0)
    (bind _asplayer_character_tapis_4 (Utilities|Casting|CastToPlayerCharacter_Tapis _returnvalue))
    (Variables|/Game/Blueprints/Player/PlayerCharacter_Tapis.PlayerCharacter_Tapis_C|SetIsinCinematic _asplayer_character_tapis_4 false)
    (Input|EnableInput (Game|GetPlayerCharacter 0) (Game|GetPlayerController 0))
    (Variables|Default|SetCutscene false)
    (else
      (Pawn|Components|CharacterMovement|SetMovementMode (Variables|/Script/Engine.Character|GetCharacterMovement (Game|GetPlayerCharacter 0)) "MOVE_Walking" 0)
      (Components|DestroyComponent (Variables|Default|GetRavenStone))
      (Variables|Default|SetTaken true)
      (bind _asgame_mode_tapis (Utilities|Casting|CastToGameMode_Tapis (Game|GetGameMode)))
      (Variables|/Game/Blueprints/GameMode_Tapis.GameMode_Tapis_C|SetAlert _asgame_mode_tapis true)
      (bind _asplayer_character_tapis_5 (Utilities|Casting|CastToPlayerCharacter_Tapis (Game|GetPlayerCharacter 0)))
      (Variables|/Game/Blueprints/Player/PlayerCharacter_Tapis.PlayerCharacter_Tapis_C|SetPromptQuitted _asplayer_character_tapis_5 false)
      (Actor|Tick|SetActorTickEnabled false)
      (Components|DestroyComponent (Variables|Default|GetItemWidget)))))

(fn ConstructionScript
  (|CallParentFunction))