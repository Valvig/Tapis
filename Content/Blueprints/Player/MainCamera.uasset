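; Player camera manager that follows the player character at a set height, pitch and FOV within bounded X and Y limits.
; BlueprintUpdateCamera casts the camera target to PlayerController_Tapis, then clamps the character's location, with an offset on X, to position the camera.
; When Y sits at either limit, yaw eases toward that side's angle with FInterpTo, otherwise back toward the start yaw.
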(fn ConstructionScript)

(fn BlueprintUpdateCamera
  (params (CameraTarget :type Actor%20Object%20Reference))
  (bind _asplayer_controller_tapis (Utilities|Casting|CastToPlayerController_Tapis CameraTarget))
  (if (> (.y (Transformation|GetActorLocation (Game|GetPlayerCharacter (Class|GameplayStatics|GetPlayerControllerID _asplayer_controller_tapis)))) (Variables|Default|GetMaxYPosition))
    (Variables|Default|SetYPosition (Variables|Default|GetMaxYPosition))
    (elif (< (.y (Transformation|GetActorLocation (Game|GetPlayerCharacter (Class|GameplayStatics|GetPlayerControllerID _asplayer_controller_tapis)))) (Variables|Default|GetMinYPosition))
      (Variables|Default|SetYPosition (Variables|Default|GetMinYPosition))
      (else
        (Variables|Default|SetYPosition (.y (Transformation|GetActorLocation (Game|GetPlayerCharacter (Class|GameplayStatics|GetPlayerControllerID _asplayer_controller_tapis))))))))
  (if (> (+ (.x (Transformation|GetActorLocation (Game|GetPlayerCharacter (Class|GameplayStatics|GetPlayerControllerID _asplayer_controller_tapis)))) (Variables|Default|GetXOffset)) (Variables|Default|GetMaxXPosition))
    (Variables|Default|SetXPosition (Variables|Default|GetMaxXPosition))
    (elif (< (+ (.x (Transformation|GetActorLocation (Game|GetPlayerCharacter (Class|GameplayStatics|GetPlayerControllerID _asplayer_controller_tapis)))) (Variables|Default|GetXOffset)) (Variables|Default|GetMinXPosition))
      (Variables|Default|SetXPosition (Variables|Default|GetMinXPosition))
      (else
        (Variables|Default|SetXPosition (+ (.x (Transformation|GetActorLocation (Game|GetPlayerCharacter (Class|GameplayStatics|GetPlayerControllerID _asplayer_controller_tapis)))) (Variables|Default|GetXOffset))))))
  (if (== (Variables|Default|GetYPosition) (Variables|Default|GetMaxYPosition))
    (Variables|Default|SetCameraYaw (Math|Interpolation|FInterpTo (.yaw (Transformation|GetActorRotation (Game|GetPlayerCameraManager (Class|GameplayStatics|GetPlayerControllerID _asplayer_controller_tapis)))) (Variables|Default|GetMaxCameraYaw) (Utilities|Time|GetWorldDeltaSeconds) (Variables|Default|GetInterpSpeed)))
    (elif (== (Variables|Default|GetYPosition) (Variables|Default|GetMinYPosition))
      (Variables|Default|SetCameraYaw (Math|Interpolation|FInterpTo (.yaw (Transformation|GetActorRotation (Game|GetPlayerCameraManager (Class|GameplayStatics|GetPlayerControllerID _asplayer_controller_tapis)))) (Variables|Default|GetMinCameraYaw) (Utilities|Time|GetWorldDeltaSeconds) (Variables|Default|GetInterpSpeed)))
      (else
        (Variables|Default|SetCameraYaw (Math|Interpolation|FInterpTo (.yaw (Transformation|GetActorRotation (Game|GetPlayerCameraManager (Class|GameplayStatics|GetPlayerControllerID _asplayer_controller_tapis)))) (Variables|Default|GetStartYaw) (Utilities|Time|GetWorldDeltaSeconds) (Variables|Default|GetInterpSpeed))))))
  (return (Math|Vector|MakeVector (Variables|Default|GetXPosition) (Variables|Default|GetYPosition) (Variables|Default|GetZPosition)) (Math|Rotator|MakeRotator 0.0 (Variables|Default|GetCameraAngle) (Variables|Default|GetCameraYaw)) (Variables|Default|GetCameraFOV) true))