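; Game mode Blueprint that runs a run timer and adds a DisplayTimer widget to the first player's viewport on BeginPlay.
; Tick sets Timer to game time minus a stored NegativeTime offset.
; ResetTimer prints the last run's time and moves the offset to the current game time.
; A disconnected snippet shows the cast-and-call pattern for triggering the reset from elsewhere.
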(event Custom|ResetTimer
  ;[0 0.4348 0.3865] Il faut appeler cet event pour reset le timer
  (Development|PrintString (Utilities|String|Append "Your last run timer is : " (Utilities|String|ToString(Float) (- (Utilities|Time|GetGameTimeinSeconds) (Variables|Default|GetNegativeTime)))) true true "(R=0.047505,G=1.000000,B=0.000000,A=1.000000)" 3.0)
  (Variables|Default|SetNegativeTime (Utilities|Time|GetGameTimeinSeconds)))

(event EventBeginPlay
  (bind _returnvalue (UserInterface|CreateWidget "/Game/Blueprints/Player/HUDWidgets/DisplayTimer.DisplayTimer_C" (Game|GetPlayerController 0)))
  (UserInterface|Viewport|AddtoViewport _returnvalue 0))

(event EventTick
  (params (DeltaSeconds :type Float%20%28single-precision%29))
  ;[0.7054 0 0.1173] Update le timer
  (Variables|Default|SetTimer (- (Utilities|Time|GetGameTimeinSeconds) (Variables|Default|GetNegativeTime))))

(fn ConstructionScript)