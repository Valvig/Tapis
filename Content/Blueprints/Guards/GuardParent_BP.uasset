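; Parent Blueprint for stealth guards that detect and catch the player by sight or contact, with an optional lantern variant.
; AI perception sets the state driving a distance-scaled suspicion meter, which updates blackboard chase flags and triggers capture when full.
; While awake and roughly on-screen, each tick runs an EQS query that rebuilds the procedural vision cone and updates suspicion.
; Guards also investigate bell sounds, and game-mode alerts wake or remove them.
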(event OnPerceptionUpdated(AIPerception)
  (params (UpdatedActors :type Array%20of%20Actor%20Object%20References))
  (bind _self self)
  (bind _returnvalue (AI|GetAIController _self))
  (bind _returnvalue_2 (AI|GetBlackboard _returnvalue))
  (Variables|Default|SetOverlappingActors UpdatedActors)
  (for (_array_element _array_index) (Variables|Default|GetOverlappingActors)
    (bind _asplayer_character_tapis (Utilities|Casting|CastToPlayerCharacter_Tapis _array_element))
    (if (Utilities|Enum|NotEqual(Enum) (Variables|/Game/Blueprints/Player/PlayerCharacter_Tapis.PlayerCharacter_Tapis_C|GetState _asplayer_character_tapis) "NewEnumerator1")
      (bind _info (Class|AIPerceptionComponent|GetActorsPerception (Variables|Default|GetAIPerceptionToUse) (Utilities|Array|Get(acopy) (Variables|Default|GetOverlappingActors) _array_index)))
      (if (.bsuccessfullysensed (Utilities|Array|Get(acopy) (.lastsensedstimuli _info)))
        (Variables|Default|SetCurrentState "NewEnumerator1")
        (else
          (Variables|Default|SetCurrentState "NewEnumerator0")
          (Utilities|IsValid _returnvalue_2
            (:Is%20Valid
              (if (ScalableFloat|GetValueasBool _returnvalue_2 (Variables|Default|GetMustFollow?))
                (AI|Components|Blackboard|SetValueasBool _returnvalue_2 (Variables|Default|GetLostPlayer) true)
                (AI|Components|Blackboard|SetValueasBool _returnvalue_2 (Variables|Default|GetMustFollow?) false)
                (AI|Components|Blackboard|SetValueasVector _returnvalue_2 (Variables|Default|GetLastKnownPlayerPosition) (.stimuluslocation (Utilities|Array|Get(acopy) (.lastsensedstimuli _info))))))))))))

(event OnComponentHit(CapsuleComponent)
  (params (HitComponent :type Primitive%20Component%20Object%20Reference) (OtherActor :type Actor%20Object%20Reference) (OtherComp :type Primitive%20Component%20Object%20Reference) (NormalImpulse :type Vector :default "0, 0, 0") (Hit :type Hit%20Result%20Structure%20%28by%20ref%29))
  (bind _returnvalue (Game|GetPlayerCharacter 0))
  (bind _capsulecomponent (Variables|Collision|GetCapsuleComponent))
  (bind _returnvalue_2 (Transformation|GetWorldLocation _capsulecomponent))
  (bind _returnvalue_3 (Transformation|GetActorLocation _returnvalue))
  (bind _returnvalue_4 (Math|Rotator|FindLookatRotation _returnvalue_2 _returnvalue_3))
  ;[0.5604 0 0.264] When the player hit a guard, he dies
  (bind _asplayer_character_tapis (Utilities|Casting|CastToPlayerCharacter_Tapis OtherActor))
  (if (Utilities|Enum|NotEqual(Enum) (Variables|/Game/Blueprints/Player/PlayerCharacter_Tapis.PlayerCharacter_Tapis_C|GetState _asplayer_character_tapis) "NewEnumerator1")
    (Variables|Default|SetCurrentState "NewEnumerator2")
    (Variables|Default|SetQuestionPercentage 1e+02)
    (Transformation|SetRelativeRotation _capsulecomponent (Math|Rotator|MakeRotator (.roll _returnvalue_4) (.pitch _returnvalue_4) (.yaw _returnvalue_4)) false false)
    (bind _asplayer_character_tapis_2 (Utilities|Casting|CastToPlayerCharacter_Tapis (Game|Player|GetPlayerPawn 0)))
    (Pawn|Components|CharacterMovement|SetMovementMode (Variables|Character|GetCharacterMovement) "MOVE_None" 0)
    (if (not (Variables|Default|GetCaughtPlayer))
      (Default|Caught _asplayer_character_tapis_2)
      (Variables|/Game/Blueprints/Player/PlayerCharacter_Tapis.PlayerCharacter_Tapis_C|SetCaught? _asplayer_character_tapis_2 true)
      (Variables|Default|SetArrowShoot true)
      (Variables|Default|SetCaughtPlayer true))))

(event OnPerceptionUpdated(AIPerceptionLantern)
  (params (UpdatedActors :type Array%20of%20Actor%20Object%20References))
  (bind _self self)
  (bind _returnvalue (AI|GetAIController _self))
  (bind _returnvalue_2 (AI|GetBlackboard _returnvalue))
  (Variables|Default|SetOverlappingActors UpdatedActors)
  (for (_array_element _array_index) (Variables|Default|GetOverlappingActors)
    (bind _asplayer_character_tapis (Utilities|Casting|CastToPlayerCharacter_Tapis _array_element))
    (if (Utilities|Enum|NotEqual(Enum) (Variables|/Game/Blueprints/Player/PlayerCharacter_Tapis.PlayerCharacter_Tapis_C|GetState _asplayer_character_tapis) "NewEnumerator1")
      (bind _info (Class|AIPerceptionComponent|GetActorsPerception (Variables|Default|GetAIPerceptionToUse) (Utilities|Array|Get(acopy) (Variables|Default|GetOverlappingActors) _array_index)))
      (if (.bsuccessfullysensed (Utilities|Array|Get(acopy) (.lastsensedstimuli _info)))
        (Variables|Default|SetCurrentState "NewEnumerator1")
        (else
          (Variables|Default|SetCurrentState "NewEnumerator0")
          (Utilities|IsValid _returnvalue_2
            (:Is%20Valid
              (if (ScalableFloat|GetValueasBool _returnvalue_2 (Variables|Default|GetMustFollow?))
                (AI|Components|Blackboard|SetValueasBool _returnvalue_2 (Variables|Default|GetLostPlayer) true)
                (AI|Components|Blackboard|SetValueasBool _returnvalue_2 (Variables|Default|GetMustFollow?) false)
                (AI|Components|Blackboard|SetValueasVector _returnvalue_2 (Variables|Default|GetLastKnownPlayerPosition) (.stimuluslocation (Utilities|Array|Get(acopy) (.lastsensedstimuli _info))))))))))))

(event Custom|Rotate
  (Variables|Default|SetIsRotating true))

(event Custom|StopRotate
  (Variables|Default|SetIsRotating false))

(event Custom|ResetGuard
  (Variables|Default|SetQuestionPercentage 0.0)
  (Variables|Default|SetCurrentState "NewEnumerator0")
  (Variables|Default|SetArrowShoot false)
  (Variables|Default|SetCaughtPlayer false)
  (Variables|Default|SetDidLoseSight false)
  (Variables|Default|SetIsRotating false))

(event Custom|LoseSight
  (Variables|Default|SetDidLoseSight true))

(event Custom|CreateCone
  (params (QueryInstance :type Env%20Query%20Instance%20Blueprint%20Wrapper%20Object%20Reference) (QueryStatus :type EEnvQueryStatus%20Enum :default "Processing"))
  (bind _self self)
  (bind _mustfollow_ (Variables|Default|GetMustFollow?))
  (bind _returnvalue (AI|GetAIController _self))
  (bind _returnvalue_2 (AI|GetBlackboard _returnvalue))
  (bind _output_get (Variables|Default|SetSightPoints (Class|EnvQueryInstanceBlueprintWrapper|GetResultsasLocations QueryInstance)))
  (bind (_vertices _triangles) (CallFunction|ConvertSightPointstoVertices _output_get (Variables|Default|GetVertices) (Variables|Default|GetTriangles)))
  (CallFunction|MaketheCone _vertices _triangles (Variables|Default|GetVisionCone) "/Game/Blueprints/Guards/M_Cone.M_Cone")
  (if (ScalableFloat|GetValueasBool (AI|GetBlackboard (AI|GetAIController self)) (Variables|Default|GetLostPlayer))
    _
    (elif (>= (Variables|Default|GetQuestionPercentage) 5e+01)
      (Utilities|IsValid _returnvalue_2
        (:Is%20Valid
          (AI|Components|Blackboard|SetValueasBool _returnvalue_2 _mustfollow_ true)))
      (else
        (Utilities|IsValid _returnvalue_2
          (:Is%20Valid
            (AI|Components|Blackboard|SetValueasBool _returnvalue_2 _mustfollow_ false))))))
  (if (Utilities|Enum|Equal(Enum) (Variables|Default|GetCurrentState) "NewEnumerator1")
    (if (< (Variables|Default|GetQuestionPercentage) 1e+02)
      (bind _asplayer_character_tapis (Utilities|Casting|CastToPlayerCharacter_Tapis (Game|Player|GetPlayerPawn 0)))
      (bind _info (Class|AIPerceptionComponent|GetActorsPerception (Variables|Default|GetAIPerceptionToUse) _asplayer_character_tapis))
      (Variables|Default|SetQuestionPercentage (+ (Variables|Default|GetQuestionPercentage) (* (Variables|Default|GetDeltaSeconds) (* (- 1e+02 (/ (* (Math|Vector|VectorLength (- (Transformation|GetActorLocation) (Transformation|GetActorLocation (.target _info)))) 1e+02) (Variables|Default|GetPerceptionRadius))) (Variables|Default|GetRateDifficulty)))))
      (else
        (Variables|Default|SetCurrentState "NewEnumerator2")
        (Variables|Default|SetQuestionPercentage 1e+02)
        (bind _asplayer_character_tapis_2 (Utilities|Casting|CastToPlayerCharacter_Tapis (Game|Player|GetPlayerPawn 0) :!label _label))
        (Pawn|Components|CharacterMovement|SetMovementMode (Variables|Character|GetCharacterMovement) "MOVE_None" 0)
        (if (not (Variables|Default|GetCaughtPlayer))
          (Default|Caught _asplayer_character_tapis_2)
          (Variables|/Game/Blueprints/Player/PlayerCharacter_Tapis.PlayerCharacter_Tapis_C|SetCaught? _asplayer_character_tapis_2 true)
          (Variables|Default|SetArrowShoot true)
          (Variables|Default|SetCaughtPlayer true))))
    (elif (Utilities|Enum|Equal(Enum) (Variables|Default|GetCurrentState) "NewEnumerator0")
      (if (> (Variables|Default|GetQuestionPercentage) 0.0)
        (Variables|Default|SetQuestionPercentage (- (Variables|Default|GetQuestionPercentage) (* (Variables|Default|GetDeltaSeconds) 1e+01)))
        (else
          (Variables|Default|SetQuestionPercentage 0.0)
          (Variables|Default|SetCurrentState "NewEnumerator0")))
      (elif (Utilities|Enum|Equal(Enum) (Variables|Default|GetCurrentState) "NewEnumerator2")
        (if (< (Variables|Default|GetQuestionPercentage) 1e+02)
          (Variables|Default|SetCurrentState "NewEnumerator1")
          (else
            (goto _label)))))))

(event Custom|StopQuestionning
  (Variables|Default|SetDidLoseSight false))

(event Custom|ReactToSound
  (params (BellLocation :type Bell%20with%20Range%20BP%20Object%20Reference))
  (bind _returnvalue (Utilities|Name|MakeLiteralName "Index"))
  (bind _returnvalue_2 (Utilities|Name|MakeLiteralName "Index"))
  (bind _self self)
  (bind _returnvalue_3 (AI|GetBlackboard _self))
  ;[0 0.08696 0.7343] REACT TO SOUND
  (Math|Float|CompareFloat (Variables|Default|GetQuestionPercentage) 5e+01
    (:==
      _)
    (:<
      _))
  (Math|Integer|CompareInt (Utilities|Map|Length (Variables|Default|GetTargetPoints))
    (:>
      ;;[0.4058 0.4155 0] If guard has at least 1 target point
      (Math|Integer|CompareInt (Class|BlackboardComponent|GetValueasInt (AI|GetBlackboard self) _returnvalue)
        (:>
          (bind _result (Math|Integer|DecrementInt (Class|BlackboardComponent|GetValueasInt _returnvalue_3 _returnvalue_2))
            (:%20%20
              (Class|BlackboardComponent|SetValueasInt _returnvalue_3 _returnvalue_2 _result))))
        (:==
          (Class|BlackboardComponent|SetValueasInt (AI|GetBlackboard self) _returnvalue (- (Utilities|Map|Length (Variables|Default|GetTargetPoints)) 1))))
      ;;;[0.06764 0.7537 0] Go check sound then go back to last target point
      (AI|AIMoveTo (AI|GetAIController self) "0, 0, 0" BellLocation 3.0 "Default" "Default" true true
        (:OnMoveFinished
          (Pawn|Components|CharacterMovement|SetMovementMode (Variables|Character|GetCharacterMovement) "MOVE_None" 0)
          (Utilities|FlowControl|Delay (Variables|Default|GetTimeDelayWhenCheckingBell))
          (Pawn|Components|CharacterMovement|SetMovementMode (Variables|Character|GetCharacterMovement) "MOVE_Walking" 0))))
    (:==
      ;;[0 0.7923 0.02899] If guard has 0 target point
      (Variables|Default|SetSavedRotationBeforeSound (Transformation|GetActorRotation) :!label _label)
      (Variables|Default|SetSavedPositionBeforeSound (Transformation|GetActorLocation))
      ;;;[0.06764 0.7537 0] Go check sound
      (AI|AIMoveTo (AI|GetAIController self) "0, 0, 0" BellLocation 3.0 "Default" "Default" true true
        (:OnMoveFinished
          (Pawn|Components|CharacterMovement|SetMovementMode (Variables|Character|GetCharacterMovement) "MOVE_None" 0)
          (Utilities|FlowControl|Delay (Variables|Default|GetTimeDelayWhenCheckingBell))
          (Pawn|Components|CharacterMovement|SetMovementMode (Variables|Character|GetCharacterMovement) "MOVE_Walking" 0)
          ;;;[0 0.6667 0.1546] Go back to initial position
          (AI|AIMoveTo (AI|GetAIController self) (Variables|Default|GetSavedPositionBeforeSound) 0 1e+01 "Default" "Default" true true
            (:OnMoveFinished
              (Pawn|Components|CharacterMovement|SetMovementMode (Variables|Character|GetCharacterMovement) "MOVE_None" 0)
              (Transformation|SetActorRotation (Variables|Default|GetSavedRotationBeforeSound))
              (Pawn|Components|CharacterMovement|SetMovementMode (Variables|Character|GetCharacterMovement) "MOVE_Walking" 0))))))
    (:<
      (goto _label))))

(event Custom|StartShoot
  (Development|SetHiddeninGame (Variables|Default|GetCrossBow) false false))

(event Custom|StopShoot
  (Rendering|SetVisibility (Variables|Default|GetCrossBow) false false)
  (Variables|Default|SetArrowShoot false))

(event Custom|SetRotationCrossBow
  (bind _crossbow (Variables|Default|GetCrossBow))
  (bind _relativerotation (Variables|/Script/Engine.SceneComponent|GetRelativeRotation _crossbow))
  (Transformation|SetRelativeRotation _crossbow (Math|Rotator|MakeRotator (.roll _relativerotation) (- (.pitch (Math|Rotator|FindLookatRotation (Transformation|GetWorldLocation _crossbow) (Transformation|GetActorLocation (Game|GetPlayerCharacter 0)))) 2e+01) (.yaw _relativerotation)) false false))

(event EventTick
  (params (DeltaSeconds :type Float%20%28single-precision%29))
  (bind _returnvalue (Game|GetPlayerController 0))
  (bind _returnvalue_2 (Transformation|GetActorLocation))
  (bind _returnvalue_3 (Viewport|GetViewportSize))
  (bind _screenlocation (Class|PlayerController|ProjectWorldLocationtoScreen _returnvalue _returnvalue_2 false))
  (bind _asgame_mode_tapis (Utilities|Casting|CastToGameMode_Tapis (Game|GetGameMode)))
  (if (Variables|/Game/Blueprints/GameMode_Tapis.GameMode_Tapis_C|GetAlert _asgame_mode_tapis)
    (if (Variables|Default|GetWillSleep)
      (Actor|DestroyActor)
      (else
        (Variables|Default|SetIsAsleep? false)
        (Development|SetHiddeninGame (Variables|Collision|GetCapsuleComponent) false true)
        (Development|SetHiddeninGame (Variables|Collision|GetCapsuleComponent) true false)
        (Collision|SetCollisionEnabled (Variables|Collision|GetCapsuleComponent) "QueryAndPhysics")
        (if (not (Variables|Default|GetIsAsleep?)) :!label _label
          (Variables|Default|SetDeltaSeconds DeltaSeconds)
          ;[0.08696 0 0.7431] Optimisation si le garde + son cône de vision ne sont pas dans l'écran
          (if (Math|Boolean|ANDBoolean (> (.x _screenlocation) 0.0) (> (.y _screenlocation) 0.0) (< (.y _screenlocation) (+ (.x _returnvalue_3) 6e+02)) (< (.y _screenlocation) (+ (.y _returnvalue_3) 6e+02)))
            (Transformation|SetWorldRotation (Variables|Default|GetWidget) "0.000000,180.000000,0.000000" false false)
            (bind _returnvalue_4 (AI|EQS|RunEQSQuery (Variables|Default|GetEnvQueryType) self "AllMatching"))
            (EventDispatchers|BindEventtoOnQueryFinishedEvent _returnvalue_4 (delegate Custom|CreateCone))))))
    (else
      (goto _label))))

(event EventBeginPlay
  (bind _targetpoints (Variables|Default|GetTargetPoints))
  (bind _aiperceptionlantern (Variables|Default|GetAIPerceptionLantern))
  (bind _aiperception (Variables|Default|GetAIPerception))
  (if (== (Utilities|Map|Length _targetpoints) 0)
    (bind _returnvalue (Game|SpawnActorfromClass "/Script/Engine.TargetPoint" (Transformation|GetWorldTransform (Variables|Collision|GetCapsuleComponent self)) "AlwaysSpawn" 0 0))
    (Utilities|Map|Add _targetpoints _returnvalue false))
  (Development|SetHiddeninGame (Variables|Default|GetCrossBow) true false)
  (if (Variables|Default|GetHasLantern)
    (Components|DestroyComponent _aiperception)
    (Variables|Default|SetAIPerceptionToUse _aiperceptionlantern)
    (else
      (Components|DestroyComponent _aiperceptionlantern)
      (Components|DestroyComponent (Variables|Default|GetLantern))
      (Variables|Default|SetAIPerceptionToUse _aiperception)))
  (Variables|/Script/Engine.CharacterMovementComponent|SetMaxWalkSpeed (Variables|Character|GetCharacterMovement self) (Variables|Default|GetNewWalkSpeed))
  (if (Variables|Default|GetIsAsleep?)
    (Development|SetHiddeninGame (Variables|Collision|GetCapsuleComponent) true true)
    (Collision|SetCollisionEnabled (Variables|Collision|GetCapsuleComponent) "NoCollision"))
  (Utilities|Array|Resize (Variables|Default|GetVertices) (+ (Variables|Default|GetNumberOfPointsCone) 1))
  (bind _asenemy_state_widget (Utilities|Casting|CastToEnemyStateWidget (UserInterface|GetUserWidgetObject (Variables|Default|GetWidget))))
  (Variables|/Game/Blueprints/Guards/Widgets/EnemyStateWidget.EnemyStateWidget_C|SetOwner _asenemy_state_widget self)
  (Variables|/Game/Blueprints/Guards/Widgets/EnemyStateWidget.EnemyStateWidget_C|SetEnemyState _asenemy_state_widget (Variables|Default|GetCurrentState)))

(fn ConstructionScript
  (if (Variables|Default|GetHasLantern)
    (Components|SkeletalMesh|SetAnimInstanceClass (Variables|Character|GetMesh) "/Game/Blueprints/Guards/aBP_GuardsLamp.aBP_GuardsLamp_C")
    (Variables|Default|SetEnvQueryType "/Game/Blueprints/Guards/ConeOfVisionGuardLantern.ConeOfVisionGuardLantern")
    (Variables|Default|SetPerceptionRadius 6e+02)
    (else
      (Components|SkeletalMesh|SetAnimInstanceClass (Variables|Character|GetMesh) "/Game/Blueprints/Guards/aBP_Guards.aBP_Guards_C")
      (Variables|Default|SetEnvQueryType "/Game/Blueprints/Guards/ConeOfVisionGuard.ConeOfVisionGuard")
      (Variables|Default|SetPerceptionRadius 5e+02))))

(fn ConvertSightPointstoVertices
  (params (SightPoints :type Array%20of%20Vectors) (VerticesEnter :type Array%20of%20Vectors) (TrianglesEnter :type Array%20of%20Integers))
  (bind _returnvalue (Utilities|Array|Length VerticesEnter))
  (bind _returnvalue_2 (Transformation|GetActorLocation))
  (bind (_x _y) (Math|Vector|BreakVector _returnvalue_2))
  (Utilities|Array|SetArrayElem :TargetArray VerticesEnter)
  (for (_array_element _array_index) SightPoints
    (Utilities|Array|SetArrayElem VerticesEnter (+ _array_index 1) (Math|Vector|MakeVector (- (.X (Math|Vector|BreakVector _array_element)) _x) (- (.Y (Math|Vector|BreakVector _array_element)) _y) 0.0)))
  (Utilities|Array|Resize TrianglesEnter (* _returnvalue 3))
  (for _index (range 0 _returnvalue)
    (Utilities|Array|SetArrayElem TrianglesEnter (* _index 3) 0)
    (Utilities|Array|SetArrayElem TrianglesEnter (+ (* _index 3) 1) (+ _index 1))
    (Utilities|Array|SetArrayElem TrianglesEnter (+ (+ (* _index 3) 1) 1) (+ (+ _index 1) 1)))
  (return VerticesEnter TrianglesEnter))

(fn MaketheCone
  (params (Vertices :type Array%20of%20Vectors) (Triangles :type Array%20of%20Integers) (VisionCone :type Procedural%20Mesh%20Component%20Object%20Reference) (Material :type Material%20Interface%20Object%20Reference))
  (Class|ProceduralMeshComponent|CreateMeshSectionLinearColor VisionCone 0 Vertices Triangles 0 0 0 0 0 0 0 false)
  (Rendering|Material|SetMaterial VisionCone 0 Material)
  (Transformation|SetWorldRotation VisionCone "0, 0, 0" false false))