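; Guard Blueprint that adds a second cone of vision, drawn as a procedural mesh, to its parent class.
; Each tick runs an EQS query from the guard, converts the resulting locations to vertices and triangles, and rebuilds the cone mesh with zero world rotation.
; A separate AI perception component sets IsQuestionning from the first updated actor's first stimulus and prints the state.
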(event OnPerceptionUpdated(AIPerceptionSecondCone)
  (params (UpdatedActors :type Array%20of%20Actor%20Object%20References))
  (bind _info (Class|AIPerceptionComponent|GetActorsPerception (Variables|Default|GetAIPerceptionSecondCone) (Utilities|Array|Get(acopy) UpdatedActors)))
  (bind _output_get (Variables|Default|SetIsQuestionning? (.bsuccessfullysensed (Utilities|Array|Get(acopy) (.lastsensedstimuli _info)))))
  (Development|PrintString (Utilities|String|Append "Am i questionning myself ? " (Utilities|String|ToString(Boolean) _output_get))))

(event Custom|CreateSecondCone
  (params (QueryInstance :type Env%20Query%20Instance%20Blueprint%20Wrapper%20Object%20Reference) (QueryStatus :type EEnvQueryStatus%20Enum :default "Processing"))
  (bind _output_get (Variables|Default|SetSecondConeSightPoints (Class|EnvQueryInstanceBlueprintWrapper|GetResultsasLocations QueryInstance)))
  (bind (_vertices _triangles) (CallFunction|ConvertSightPointstoVertices _output_get (Variables|Default|GetSecondConeVertices) (Variables|Default|GetSecondConeTriangles)))
  (CallFunction|MaketheSecondCone _vertices _triangles))

(event EventBeginPlay
  (Utilities|Array|Resize (Variables|Default|GetSecondConeVertices) (+ (Variables|Default|GetNumberOfPointsSecondCone) 1)))

(event EventTick
  (params (DeltaSeconds :type Float%20%28single-precision%29))
  (bind _returnvalue (AI|EQS|RunEQSQuery "/Game/Blueprints/Guards/GuardDoubleVision/SecondConeOfVisionGuard.SecondConeOfVisionGuard" self "AllMatching"))
  (EventDispatchers|BindEventtoOnQueryFinishedEvent _returnvalue (delegate Custom|CreateSecondCone)))

(fn ConstructionScript
  (|CallParentFunction))

(fn MaketheSecondCone
  (params (Vertices :type Array%20of%20Vectors) (Triangles :type Array%20of%20Integers))
  (bind _secondvisioncone (Variables|Default|GetSecondVisionCone))
  (Class|ProceduralMeshComponent|CreateMeshSectionLinearColor _secondvisioncone 0 Vertices Triangles 0 0 0 0 0 0 0 false)
  (Rendering|Material|SetMaterial _secondvisioncone 0 "/Game/Geometry/Meshes/CubeMaterial.CubeMaterial")
  (Transformation|SetWorldRotation _secondvisioncone "0, 0, 0" false false))